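; BP_Diamond_Auto1 is a collectible diamond that the nfrtBLP2 actor picks up by touching it.
; On overlap with the Diamond component, it calls AddDiamonds on that actor, plays a ping at its location and destroys itself.
; A SpawnDiamonds function adds a child actor component at a random point inside the DiamondCollision box, but nothing in this Blueprint calls it.
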(event `self.ReceiveBeginPlay`)

(event `self.ReceiveActorBeginOverlap`
  (params (OtherActor :type "Actor Object Reference")))

(event `self.ReceiveTick`
  (params (DeltaSeconds :type "Float (single-precision)")))

(event `self.Diamond.OnComponentBeginOverlap`
  (params (OtherActor :type "Actor Object Reference") (OtherComp :type "PrimitiveComponent Object Reference") (OtherBodyIndex :type Integer) (bFromSweep :type Boolean) (SweepResult :type "HitResult Structure (by ref)"))
  (bind _asnfrt_blp2 (cast `/Game/Vehicles/nfrt6/nfrtBLP2` OtherActor))
  (`/Game/Vehicles/nfrt6/nfrtBLP2.AddDiamonds` _asnfrt_blp2)
  (`GameplayStatics.PlaySoundAtLocation` "/Game/Content/BP_Diamond/Ping_-_Sound_Effect.Ping_-_Sound_Effect" (`self.K2_GetActorLocation`))
  (`self.K2_DestroyActor`))

(fn `SpawnDiamonds`
  (bind _diamondcollision (`self.DiamondCollision`))
  (`AddComponent|Child Actor Component_6912` :`RelativeTransform` (`KismetMathLibrary.Conv_VectorToTransform` (`KismetMathLibrary.RandomPointInBoundingBox` (`SceneComponent.RelativeLocation` _diamondcollision) (`BoxComponent.BoxExtent` _diamondcollision)))))

(fn `UserConstructionScript`)