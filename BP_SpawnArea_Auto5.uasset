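; BP_SpawnArea_Auto5 is a spawn area piece that scatters coins and exposes an attach point transform, likely for chaining pieces.
; The construction script calls SpawnCoins, which adds child actor components at random points inside the CoinArea box.
; GetAttachTransform returns AttachPoint's world transform.
; SetSpawnPoints is empty, its left/right/center spawn-point array is disconnected, and the random branch after it does nothing.
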(event `self.ReceiveBeginPlay`)

(event `self.ReceiveActorBeginOverlap`
  (params (OtherActor :type "Actor Object Reference")))

(event `self.ReceiveTick`
  (params (DeltaSeconds :type "Float (single-precision)")))

(fn `GetAttachTransform`
  (returns (AttachTransform :type "Transform Structure"))
  (return (`SceneComponent.K2_GetComponentToWorld` (`self.AttachPoint`))))

(fn `SetSpawnPoints`)

(fn `SpawnCoins`
  (bind _coinarea (`self.CoinArea`))
  (for _ (range 31)
    (`AddComponent|Child Actor Component_1` :`RelativeTransform` (`KismetMathLibrary.Conv_VectorToTransform` (`KismetMathLibrary.RandomPointInBoundingBox` (`SceneComponent.RelativeLocation` _coinarea) (`BoxComponent.BoxExtent` _coinarea))))))

(fn `UserConstructionScript`
  (`self.SetSpawnPoints`)
  (switch `int` (`KismetMathLibrary.RandomIntegerInRange` 0 1)
    (:`Default`
      _)
    (:`0`
      _))
  (`self.SpawnCoins`))