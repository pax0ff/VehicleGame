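; Spawn-area actor that scatters diamond pickups as child actors at random points inside its SpawnArea box.
; The construction script runs a fixed-count SpawnDiamonds loop, so placement is re-randomised whenever construction reruns.
; GetAttachTransform exposes the AttachPoint world transform to callers.
; SetSpawnPoints and the random branch do nothing, the left/centre/right spawn-point array code is disconnected, and the event graph is empty.
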(event `self.ReceiveBeginPlay`)

(event `self.ReceiveActorBeginOverlap`
  (params (OtherActor :type "Actor Object Reference")))

(event `self.ReceiveTick`
  (params (DeltaSeconds :type "Float (single-precision)")))

(fn `GetAttachTransform`
  (returns (AttachTransform :type "Transform Structure"))
  (return (`SceneComponent.K2_GetComponentToWorld` (`self.AttachPoint`))))

(fn `SetSpawnPoints`)

(fn `SpawnDiamonds`
  (bind _spawnarea (`self.SpawnArea`))
  (for _ (range 26)
    (`AddComponent|Child Actor Component_751` :`RelativeTransform` (`KismetMathLibrary.Conv_VectorToTransform` (`KismetMathLibrary.RandomPointInBoundingBox` (`SceneComponent.RelativeLocation` _spawnarea) (`BoxComponent.BoxExtent` _spawnarea))))))

(fn `UserConstructionScript`
  (`self.SetSpawnPoints`)
  (switch `int` (`KismetMathLibrary.RandomIntegerInRange` 0 1)
    (:`Default`
      _)
    (:`0`
      _))
  (`self.SpawnDiamonds`))