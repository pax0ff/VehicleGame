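; BP_Projectile_Auto1 is a Blueprint that spawns BP_Projectile actors.
; Pressing the right mouse button spawns one at the Projectile component's world location and rotation, ignoring collisions.
; A separate FirePRJ function, not called in this graph, spawns one offset from the actor's location.
; Its direction derives from the actor's world position vector rather than the actor's rotation.
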(event `Key|RightMouseButton`
  (params (Key :type "Key Structure" :default "AnyKey"))
  (bind _projectile (`self.Projectile`))
  (:`Pressed`
    (`|SpawnActorFromClass` "BP_Projectile_C" (`KismetMathLibrary.MakeTransform` (`SceneComponent.K2_GetComponentLocation` _projectile) (`SceneComponent.K2_GetComponentRotation` _projectile)) "AlwaysSpawn" "OverrideRootScale")))

(event `self.ReceiveBeginPlay`)

(event `self.ReceiveActorBeginOverlap`
  (params (OtherActor :type "Actor Object Reference")))

(event `self.ReceiveTick`
  (params (DeltaSeconds :type "Float (single-precision)")))

(fn `FirePRJ`
  (bind _returnvalue (`KismetMathLibrary.Conv_VectorToRotator` (`self.K2_GetActorLocation`)))
  (`|SpawnActorFromClass` "BP_Projectile_C" (`KismetMathLibrary.MakeTransform` (+ (`self.K2_GetActorLocation`) (* (`KismetMathLibrary.GetForwardVector` _returnvalue) 500.0)) _returnvalue) "Undefined" "OverrideRootScale"))

(fn `UserConstructionScript`)